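; BP_GameModePlatform is the game mode for the platform game, tracking player health and a money count.
; On BeginPlay it adds score and health bar widgets to the viewport, keeping a reference only to the health bar.
; Hit and life-gain events adjust Hp by a fixed step, capping only at HpMax, then UpdateUI sends the health ratio to the bar.
; AddMoney just increments the counter, without refreshing any UI.
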(event Custom|OnHitPlayer
  (Variables|Default|Sethp (- (Variables|Default|Gethp) 1e+01))
  (CallFunction|UpdateUI))

(event Custom|OnGainLife
  (bind _output_get (Variables|Default|Sethp (+ (Variables|Default|Gethp) 1e+01)))
  (if (>= _output_get (Variables|Default|GethpMax))
    (Variables|Default|Sethp (Variables|Default|GethpMax)))
  (CallFunction|UpdateUI))

(event EventBeginPlay
  (bind _returnvalue (UserInterface|CreateWidget "/Game/Blueprints/Platform/WBP_ScorePlatform.WBP_ScorePlatform_C"))
  (UserInterface|Viewport|AddtoViewport _returnvalue 0)
  (bind _returnvalue_2 (UserInterface|CreateWidget "/Game/Blueprints/Platform/WBP_HealthBar.WBP_HealthBar_C"))
  (bind _output_get (Variables|Default|SetPanelHealthBar _returnvalue_2))
  (UserInterface|Viewport|AddtoViewport _output_get 0))

(fn ConstructionScript)

(fn AddMoney
  (Math|Integer|IncrementInt (Variables|Default|GetMoneyCount)))

(fn UpdateUI
  (Default|UpdateBar (Variables|Default|GetPanelHealthBar) (/ (Variables|Default|Gethp) (Variables|Default|GethpMax))))